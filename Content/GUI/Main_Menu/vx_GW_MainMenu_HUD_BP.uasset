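; Main menu HUD that puts up the menu UI and manages cursor and input mode while the player is in it.
; On BeginPlay it creates a base layout widget, adds it to the viewport, pushes the main menu onto it, then shows the cursor and switches to UI-only input.
; An opening level-transition event hides the menu widget and, if the cursor is showing, hides it and returns input to game-only.
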(event `self.ReceiveBeginPlay`
  (bind _returnvalue (`GameplayStatics.GetPlayerController` 0))
  (`|ExecutionSequence`
    (:`then_0`
      (bind _returnvalue_2 (`|CreateWidget` (`self.Base_Layout`) (`self.PlayerOwner`)))
      (bind _asvx_gw_main_menu_2 (cast `/Game/GUI/Main_Menu/Widgets/vx_GW_Base_Layout` _returnvalue_2))
      (bind _output_get (set `self.Base Layout` _asvx_gw_main_menu_2))
      (`UserWidget.AddToViewport` _output_get 0)
      (`/Game/GUI/Main_Menu/Widgets/vx_GW_Base_Layout.PushWidget` _output_get "/Game/GUI/Main_Menu/Widgets/vx_Main_Menu.vx_Main_Menu_C"))
    (:`then_1`
      (if (not (`PlayerController.bShowMouseCursor` (`GameplayStatics.GetPlayerController` 0)))
        (set `PlayerController.bShowMouseCursor` true _returnvalue))
      (`WidgetBlueprintLibrary.SetInputMode_UIOnlyEx` _returnvalue (`self.vx_Main_Menu_Widget`)))))

(event `vx Opening Transirion Level`
  (bind _returnvalue (`GameplayStatics.GetPlayerController` 0))
  (`Widget.SetVisibility` (`self.vx_Main_Menu_Widget`) "Hidden")
  (if (`PlayerController.bShowMouseCursor` (`GameplayStatics.GetPlayerController` 0))
    (set `PlayerController.bShowMouseCursor` false _returnvalue)
    (`WidgetBlueprintLibrary.SetInputMode_GameOnly` _returnvalue)))

(fn `UserConstructionScript`
  (`parent.UserConstructionScript`))