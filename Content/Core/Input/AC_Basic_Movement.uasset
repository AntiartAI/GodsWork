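; AC_Basic_Movement is a component that handles basic player jump and look input for its character.
; On BeginPlay it links the IMC_vx_Basic_Movement mapping context to the player controller, overriding any existing one.
; The jump action sets a Jump flag and calls Jump on the character's ExtendedCharacterMoverComponent, clearing the flag on completion.
; The look action feeds controller yaw and pitch; no directional movement is handled here.
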(event `Init Input Mapping`
  (`/Game/Core/Input/BFL_Intput.vx_Link Input Mapping` false (`/Game/Core/Input/BML_Generic_Component.Get Player Controller`) "/Game/Core/Input/Basic_Movement/IMC_vx_Basic_Movement.IMC_vx_Basic_Movement" 0 true))

(event `self.ReceiveBeginPlay`
  (`parent.ReceiveBeginPlay`)
  (`self.Init Input Mapping`))

(event `EnhancedInput|/Game/Core/Input/Basic_Movement/IA_vx_Jump`
  (params (ActionValue :type Boolean) (ElapsedSeconds :type "Float (double-precision)") (TriggeredSeconds :type "Float (double-precision)") (InputAction :type "InputAction Object Reference" :default "/Game/Core/Input/Basic_Movement/IA_vx_Jump.IA_vx_Jump"))
  (:`Triggered`
    (set `self.Jump` true)
    (`CharacterMoverComponent.Jump` (`/Game/Player_Characters/vx_TestCharacter/vx_MoverExample_Character.ExtendedCharacterMoverComponent` (`/Game/Core/Input/BML_Generic_Component.Get CHaracter`))))
  (:`Completed`
    (set `self.Jump` false)))

(event `EnhancedInput|/Game/Core/Input/Basic_Movement/IA_vx_Look`
  (params (ActionValue :type "Vector2D Structure") (ElapsedSeconds :type "Float (double-precision)") (TriggeredSeconds :type "Float (double-precision)") (InputAction :type "InputAction Object Reference" :default "/Game/Core/Input/Basic_Movement/IA_vx_Look.IA_vx_Look"))
  (bind _character (`/Game/Core/Input/BML_Generic_Component.Get CHaracter`))
  (:`Triggered`
    (`Pawn.AddControllerYawInput` _character ActionValue_X)
    (`Pawn.AddControllerPitchInput` _character ActionValue_Y)))