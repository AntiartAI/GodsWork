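; Base game mode Blueprint that prints debug messages for player connections and departures and overrides login approval.
; OnPlayerJoined binds a handler to the player-connected event that prints the new player's name.
; OnPlayerLeft prints a goodbye with the leaving controller's name, then binds an empty disconnect handler.
; ApprovePlayerLogin always returns true, despite also setting a "not welcome" reject reason.
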(event `self.OnPlayerJoined`
  (params (NewPlayer :type "PlayerController Object Reference"))
  (add `self.OnPlayerConnected` (delegate `CustomEvent`)))

(event `CustomEvent` :!signature `self.OnPlayerConnected`
  (params (NewPlayer :type "PlayerController Object Reference"))
  (`KismetSystemLibrary.PrintString` (`KismetSystemLibrary.GetDisplayName` NewPlayer) true true (struct :`G` 1.0 :`B` 0.011908 :`A` 1.0) 5.0))

(event `self.OnPlayerLeft`
  (params (ExitingController :type "Controller Object Reference"))
  (`KismetSystemLibrary.PrintString` (`KismetStringLibrary.Concat_StrStr` "BuBye" (`KismetSystemLibrary.GetDisplayName` ExitingController)) true true (struct :`R` 1.0 :`B` 0.031181 :`A` 1.0))
  (add `self.OnPlayerDisconnected` (delegate `Bye Player!!`)))

(event `Bye Player!!` :!signature `self.OnPlayerDisconnected`
  (params (ExitingController :type "Controller Object Reference")))

(fn `ApprovePlayerLogin`
  (params (Options :type String) (Address :type String) (UniqueId :type String))
  (returns (OutRejectReason :type String) (ReturnValue :type Boolean))
  (return "not welcome" true))

(fn `UserConstructionScript`)